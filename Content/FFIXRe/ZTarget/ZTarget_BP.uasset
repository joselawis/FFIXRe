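; Z-targeting lock-on actor, attached to a parent actor, that selects, highlights and locks onto targets within a configurable sphere.
; Sphere overlaps maintain the in-range list, and check events pick either the nearest target or the one closest to the camera's view line.
; An optional line trace requires visibility; locking freezes selection until toggled off, out of range or occluded.
; "Outline"-tagged meshes show highlighting through custom depth, with stencil marking locks.
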(event `self.ReceiveBeginPlay`
  (set `self.Parent` (`self.GetParentActor`))
  (`self.GetAllOverlappingTargets`))

(event `self.LockOnSphere.OnComponentBeginOverlap`
  (params (OverlappedComponent :type "PrimitiveComponent Object Reference") (OtherActor :type "Actor Object Reference") (OtherComp :type "PrimitiveComponent Object Reference") (OtherBodyIndex :type Integer) (bFromSweep :type Boolean) (SweepResult :type "HitResult Structure (by ref)"))
  (`KismetArrayLibrary.Array_Add` (`self.AllInRangeTargets`) OtherActor))

(event `self.LockOnSphere.OnComponentEndOverlap`
  (params (OverlappedComponent :type "PrimitiveComponent Object Reference") (OtherActor :type "Actor Object Reference") (OtherComp :type "PrimitiveComponent Object Reference") (OtherBodyIndex :type Integer))
  (`KismetArrayLibrary.Array_RemoveItem` (`self.AllInRangeTargets`) OtherActor) ; Remove target
  (`self.HighLightTargetOff` OtherActor)
  (if (== OtherActor (`self.CurrentTarget`))
    (set `self.IsLocked` false)))

(event `ToggleLock`
  (bind _currenttarget (`self.CurrentTarget`))
  ;[1 1 1] Toggle Locked
  (if (`self.IsLocked`)
    (set `self.IsLocked` false)
    (`self.HighLightTargetOff` _currenttarget true)
    (else
      (set `self.IsLocked` true)
      (`self.HighLightTargetOn` _currenttarget))))

(event `CheckNearestTarget`
  ;[1 1 1] Check Nearest Target
  (if (`self.IsLocked`)
    (if (`self.OnlyVisible`)
      (bind _isvisible (`self.IsVisibleTarget` (`self.CurrentTarget`)))
      (if (not _isvisible)
        (`self.HighLightTargetOff` (`self.CurrentTarget`))
        (set `self.CurrentTarget` null)
        (set `self.IsLocked` false)))
    (else
      (bind _nearesttarget (`self.GetNearestTarget`))
      (if (not (== (`self.CurrentTarget`) _nearesttarget))
        (`/Engine/EditorBlueprintResources/StandardMacros.IsValid` (`self.CurrentTarget`)
          (:`Is Valid`
            (`self.HighLightTargetOff` (`self.CurrentTarget`)))
          (:`Is Not Valid`
            _))
        (bind _output_get (set `self.CurrentTarget` _nearesttarget))
        (`self.HighLightTargetOn` _output_get)))))

(event `CheckLookingAtTarget`
  (params (CameraLocation :type "Vector Structure") (CameraVector :type "Vector Structure"))
  ;[1 1 1] Check Looking At Target
  (if (`self.IsLocked`)
    (if (`self.OnlyVisible`)
      (bind _isvisible (`self.IsVisibleTarget` (`self.CurrentTarget`)))
      (if (not _isvisible)
        (`self.HighLightTargetOff` (`self.CurrentTarget`))
        (set `self.CurrentTarget` null)
        (set `self.IsLocked` false)))
    (else
      (bind _lookingattarget (`self.GetLookingAtTarget` CameraLocation CameraVector))
      (if (not (== (`self.CurrentTarget`) _lookingattarget))
        (`/Engine/EditorBlueprintResources/StandardMacros.IsValid` (`self.CurrentTarget`)
          (:`Is Valid`
            (`self.HighLightTargetOff` (`self.CurrentTarget`)))
          (:`Is Not Valid`
            _))
        (bind _output_get (set `self.CurrentTarget` _lookingattarget))
        (`self.HighLightTargetOn` _output_get)))))

(event `LockToTarget`
  (params (InputTarget :type "Actor Object Reference"))
  (if (!= InputTarget (`self.CurrentTarget`))
    (`self.HighLightTargetOff` (`self.CurrentTarget`)))
  (bind _output_get (set `self.CurrentTarget` InputTarget))
  (`self.HighLightTargetOn` _output_get)
  (set `self.IsLocked` true))

(fn `GetAllOverlappingTargets`
  (for _array_element (`PrimitiveComponent.GetOverlappingActors` (`self.LockOnSphere`) null)
    (if (`KismetSystemLibrary.DoesImplementInterface` _array_element "/Game/FFIXRe/ZTarget/Targetable_BPI.Targetable_BPI_C")
      (`KismetArrayLibrary.Array_Add` (`self.AllInRangeTargets`) _array_element)))
  (return))

(fn `GetLookingAtTarget`
  (params (CameraLocation :type "Vector Structure") (CameraVector :type "Vector Structure"))
  (returns (LookingAtTarget :type "Actor Object Reference"))
  (locals (LowerDistance :type "Float (double-precision)") (SelectedTarget :type "Actor Object Reference"))
  (set `local.LowerDistance` (`self.LockOnRadius`))
  (for _array_element (`self.AllInRangeTargets`)
    (if (`self.OnlyVisible`)
      ;[1 1 1] If OnlyVisibles check if is visible
      (bind _isvisible (`self.IsVisibleTarget` _array_element))
      (if _isvisible
        (bind _returnvalue (`KismetMathLibrary.GetPointDistanceToLine` (`self.K2_GetActorLocation` _array_element) CameraLocation CameraVector))
        (if (< _returnvalue (`local.LowerDistance`)) :!label _label
          (set `local.LowerDistance` _returnvalue)
          (set `local.SelectedTarget` _array_element)))
      (else
        (goto _label))))
  (return (`local.SelectedTarget`)))

(fn `GetNearestTarget`
  (returns (NearestTarget :type "Actor Object Reference"))
  (locals (LowerDistance :type "Float (double-precision)") (SelectedTarget :type "Actor Object Reference"))
  (set `local.LowerDistance` (`self.LockOnRadius`))
  (for _array_element (`self.AllInRangeTargets`)
    (if (`self.OnlyVisible`)
      ;[1 1 1] If OnlyVisibles check if is visible
      (bind _isvisible (`self.IsVisibleTarget` _array_element))
      (if _isvisible
        (bind _returnvalue (`self.GetDistanceTo` _array_element))
        (if (< _returnvalue (`local.LowerDistance`)) :!label _label
          (set `local.LowerDistance` _returnvalue)
          (set `local.SelectedTarget` _array_element)))
      (else
        (goto _label))))
  (return (`local.SelectedTarget`)))

(fn `HighLightTargetOff`
  (params (Target :type "Actor Object Reference") (RenderCustomDepth :type Boolean))
  (bind _output (`|GetArrayItem` (`self.GetComponentsByTag` Target "/Script/Engine.MeshComponent" "Outline")))
  (`/Engine/EditorBlueprintResources/StandardMacros.IsValid` _output
    (:`Is Valid`
      (`PrimitiveComponent.SetRenderCustomDepth` _output RenderCustomDepth)
      (`PrimitiveComponent.SetCustomDepthStencilValue` _output 0))))

(fn `HighLightTargetOn`
  (params (Target :type "Actor Object Reference"))
  (bind _output (`|GetArrayItem` (`self.GetComponentsByTag` Target "/Script/Engine.MeshComponent" "Outline")))
  (`/Engine/EditorBlueprintResources/StandardMacros.IsValid` Target
    (:`Is Valid`
      (`PrimitiveComponent.SetRenderCustomDepth` _output true)
      (if (`self.IsLocked`)
        (`PrimitiveComponent.SetCustomDepthStencilValue` _output 1)))))

(fn `Initialize`
  (params (LockOnSphereRadius :type "Float (double-precision)"))
  (bind _output_get (set `self.LockOnRadius` LockOnSphereRadius))
  (`SphereComponent.SetSphereRadius` (`self.LockOnSphere`) _output_get true))

(fn `IsVisibleTarget`
  (params (Target :type "Actor Object Reference"))
  (returns (IsVisible :type Boolean))
  (locals (IgnoredObjects :type "Array of Actor Object Reference"))
  (`/Engine/EditorBlueprintResources/StandardMacros.IsValid` Target
    (:`Is Valid`
      (bind _output_get (set `local.IgnoredObjects` (`self.AllInRangeTargets`)))
      (`KismetArrayLibrary.Array_Add` _output_get (`self.Parent`))
      (`KismetArrayLibrary.Array_RemoveItem` (`local.IgnoredObjects`) Target)
      (bind _outhit (`KismetSystemLibrary.LineTraceSingleForObjects` (`self.K2_GetActorLocation`) (`self.K2_GetActorLocation` Target) (`|MakeArray` "ObjectTypeQuery1" "ObjectTypeQuery2" "ObjectTypeQuery3" :!type "EObjectTypeQuery Enum") false (`local.IgnoredObjects`)))
      (return (== (`.HitActor` (`GameplayStatics.BreakHitResult` _outhit)) Target)))))

(fn `UserConstructionScript`
  (`SphereComponent.SetSphereRadius` (`self.LockOnSphere`) (`self.LockOnRadius`) true))